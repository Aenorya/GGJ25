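; BP_PlayerController is the player controller that drives BP_PlayerCharacter through Enhanced Input.
; On BeginPlay it adds the input mapping context and caches the character.
; Move input pushes the character along its forward vector at BubbleSpeed and turns yaw in proportion to current velocity, so steering depends on motion.
; Fly input adds vertical movement scaled by FlySpeed, and both actions then call the character's LerpLocation.
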(event Input|EnhancedActionEvents|EnhancedInputActionInputAction_Move
  (params (ActionValue :type Vector%202D%20Structure) (ElapsedSeconds :type Float%20%28double-precision%29) (TriggeredSeconds :type Float%20%28double-precision%29) (InputAction :type Input%20Action%20Object%20Reference :default "/Game/Input/InputAction_Move.InputAction_Move"))
  (bind _returnvalue (Math|Vector2D|Normalize2D ActionValue))
  (bind _returnvalue_2 (Game|GetPlayerCharacter 0))
  (Pawn|Input|AddMovementInput _returnvalue_2 (* (.x _returnvalue) (Transformation|GetActorForwardVector _returnvalue_2)) (Variables|Default|GetbubbleSpeed) true)
  (Pawn|Input|AddControllerYawInput _returnvalue_2 (* (.y _returnvalue) (/ (Math|Vector|VectorLength (Transformation|GetVelocity (Variables|Default|GetplayerCharacter))) 1.2e+03)))
  (Default|LerpLocation (Variables|Default|GetplayerCharacter)))

(event Input|EnhancedActionEvents|EnhancedInputActionInputAction_Fly
  (params (ActionValue :type Float%20%28double-precision%29) (ElapsedSeconds :type Float%20%28double-precision%29) (TriggeredSeconds :type Float%20%28double-precision%29) (InputAction :type Input%20Action%20Object%20Reference :default "/Game/Input/InputAction_Fly.InputAction_Fly"))
  (Pawn|Input|AddMovementInput (Variables|Default|GetplayerCharacter) "0.000000,0.000000,1.000000" (* ActionValue (Variables|Default|GetflySpeed)) false)
  (Default|LerpLocation (Variables|Default|GetplayerCharacter)))

(event EventBeginPlay
  (Input|AddMappingContext (PlayerController|LocalPlayerSubsystems|GetEnhancedInputLocalPlayerSubsystem) "/Game/Input/InputMappingContext.InputMappingContext" 0 "(bIgnoreAllPressedKeysUntilRelease=True,bForceImmediately=False,bNotifyUserSettings=False)")
  (bind _asbp_player_character (Utilities|Casting|CastToBP_PlayerCharacter (Game|GetPlayerCharacter 0)))
  (Variables|Default|SetplayerCharacter _asbp_player_character))

(event EventTick
  (params (DeltaSeconds :type Float%20%28single-precision%29)))

(fn ConstructionScript)