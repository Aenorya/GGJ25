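; Player character that trails a snake-like, growable chain of bubble body parts, drawn as instances of one detached instanced static mesh.
; Construction builds the tapering chain and offsets the cine camera to suit its length.
; While moving, Tick pins the first bubble behind the actor and lerps each other toward its predecessor's snapshotted transform, eased by BubbleSpacing.
; AddBodyPart appends a scaled bubble and shifts the camera; CanGrow checks the maximum count.
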(event Custom|LerpLocation
  (bind _returnvalue (Transformation|GetActorTransform))
  (bind _bodypartscount (Variables|Default|GetBodyPartsCount))
  (bind _ism (Variables|Default|GetISM))
  (if (> _bodypartscount 0)
    (Utilities|Array|Clear (Variables|Default|GetInstanceTransform))
    (for _index (range 0 (- _bodypartscount 1))
      (Utilities|Array|Add (Variables|Default|GetInstanceTransform) (.OutInstanceTransform (Components|InstancedStaticMesh|GetInstanceTransform (Variables|Default|GetISM) _index true))))
    (Components|InstancedStaticMesh|UpdateInstanceTransform (Variables|Default|GetISM) 0 (Math|Transform|MakeTransform (- (.location _returnvalue) (* (Transformation|GetActorForwardVector) "110.000000,0.000000,50.000000")) (.rotation _returnvalue) "1.000000,1.000000,1.000000") true true false)
    (for (_array_element _array_index) (Variables|Default|GetInstanceTransform)
      (Components|InstancedStaticMesh|UpdateInstanceTransform _ism (+ _array_index 1) (Math|Transform|MakeTransform (.location (Math|Transform|Lerp(Transform) (.OutInstanceTransform (Components|InstancedStaticMesh|GetInstanceTransform _ism (+ _array_index 1) true)) _array_element (/ 1.0 (Variables|Default|GetbubbleSpacing)))) (.rotation (Math|Transform|Lerp(Transform) (.OutInstanceTransform (Components|InstancedStaticMesh|GetInstanceTransform _ism (+ _array_index 1) true)) _array_element (/ 1.0 (Variables|Default|GetbubbleSpacing)))) (.Scale (Math|Transform|BreakTransform (.OutInstanceTransform (Components|InstancedStaticMesh|GetInstanceTransform _ism (+ _array_index 1) true))))) true true false))))

(event EventBeginPlay)

(event Collision|EventActorBeginOverlap
  (params (OtherActor :type Actor%20Object%20Reference)))

(event EventTick
  (params (DeltaSeconds :type Float%20%28single-precision%29))
  (if (not (Utilities|Operators|EqualEqual :A (Transformation|GetVelocity) :ErrorTolerance 0.1))
    (CallFunction|LerpLocation)))

(fn ConstructionScript
  (bind _ism (Variables|Default|GetISM))
  (Transformation|DetachFromComponent _ism "KeepWorld" "KeepWorld" "KeepWorld" true)
  (Components|InstancedStaticMesh|ClearInstances _ism)
  (for _index (range 0 (- (Variables|Default|GetBodyPartsCount) 1))
    (Components|InstancedStaticMesh|AddInstance (Variables|Default|GetISM) (Math|Transform|MakeTransform (Math|Vector|MakeVector (Math|Conversions|ToFloat(Integer) (* _index -100)) 0.0 0.0) "0, 0, 0" (Math|Vector|MakeVector (Math|Float|Max(Float) (- 1 (* _index 0.05)) (Variables|Default|GetminBubbleScale)) (Math|Float|Max(Float) (- 1 (* _index 0.05)) (Variables|Default|GetminBubbleScale)) (Math|Float|Max(Float) (- 1 (* _index 0.05)) (Variables|Default|GetminBubbleScale)))) false))
  (Transformation|AddLocalOffset (Variables|Default|GetCineCamera) (Math|Vector|MakeVector (* (.x (.location (.OutInstanceTransform (Components|InstancedStaticMesh|GetInstanceTransform (Variables|Default|GetISM) (- (Variables|Default|GetBodyPartsCount) 1) false)))) 2.0) 0.0 0.0) false false))

(fn AddBodyPart
  (bind _ism (Variables|Default|GetISM))
  (Variables|Default|SetBodyPartsCount (+ (Variables|Default|GetBodyPartsCount) 1))
  (Components|InstancedStaticMesh|AddInstance _ism (Math|Transform|MakeTransform (.location (.OutInstanceTransform (Components|InstancedStaticMesh|GetInstanceTransform _ism (- (Variables|Default|GetBodyPartsCount) 2) false))) (.rotation (.OutInstanceTransform (Components|InstancedStaticMesh|GetInstanceTransform _ism (- (Variables|Default|GetBodyPartsCount) 2) false))) (Math|Vector|MakeVector (Math|Float|Max(Float) (- 1 (* (Math|Conversions|ToFloat(Integer) (- (Variables|Default|GetBodyPartsCount) 2)) (Variables|Default|GetscaleImpact))) (Variables|Default|GetminBubbleScale)) (Math|Float|Max(Float) (- 1 (* (Math|Conversions|ToFloat(Integer) (- (Variables|Default|GetBodyPartsCount) 2)) (Variables|Default|GetscaleImpact))) (Variables|Default|GetminBubbleScale)) (Math|Float|Max(Float) (- 1 (* (Math|Conversions|ToFloat(Integer) (- (Variables|Default|GetBodyPartsCount) 2)) (Variables|Default|GetscaleImpact))) (Variables|Default|GetminBubbleScale)))) false)
  (Transformation|AddLocalOffset (Variables|Default|GetCineCamera) (Math|Vector|MakeVector (* (Variables|Default|GetBodyPartsCount) -1e+01) 0.0 0.0) false false))

(fn CanGrow
  (return (< (+ (Variables|Default|GetBodyPartsCount) 1) (Variables|Default|GetmaxBubbleCount))))